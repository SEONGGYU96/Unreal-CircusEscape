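; BP_Kenny is a physics-driven player character that balances, jumps and dies when it tips over on the ground.
; Tilt input rotates the capsule in the air and pushes the Head on the ground, while Jump launches it along its up vector.
; Hits update IsFlying by the other actor's class, and a delayed Tick sets it back to true.
; Tick also checks inclination, ragdolling the mesh with a death sound.
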(event Collision|EventHit
  (params (MyComp :type Primitive%20Component%20Object%20Reference) (Other :type Actor%20Object%20Reference) (OtherComp :type Primitive%20Component%20Object%20Reference) (bSelfMoved :type Boolean) (HitLocation :type Vector :default "0, 0, 0") (HitNormal :type Vector :default "0, 0, 0") (NormalImpulse :type Vector :default "0, 0, 0") (Hit :type Hit%20Result%20Structure%20%28by%20ref%29))
  (Variables|Default|SetisFlying (== (Utilities|GetClass Other) "/Script/Engine.Actor")))

(event EventTick
  (params (DeltaSeconds :type Float%20%28single-precision%29))
  (CallFunction|RunDieObserver)
  (Utilities|FlowControl|Delay 0.2)
  (Variables|Default|SetisFlying true))

(event Input|ActionEvents|InputActionJump
  (params (Key :type Key%20Structure :default "None"))
  (:Pressed
    (if (not (Variables|Default|GetisFlying))
      (Variables|Default|SetisFlying true)
      (Physics|AddForce (Variables|Collision|GetCapsuleComponent) (* (Math|Vector|GetUpVector (Transformation|GetActorRotation)) 2.7e+04) "None" true)
      (Audio|PlaySoundatLocation "/Game/Kenny/Sound/CE_JumpSound.CE_JumpSound" (Transformation|GetActorLocation) "0, 0, 0" 1.0 1.0 0.0 0 0 0))))

(event Input|AxisEvents|InputAxisTilt
  (params (AxisValue :type Float%20%28single-precision%29))
  (bind _returnvalue (Transformation|GetActorRotation))
  (bind _capsulecomponent (Variables|Collision|GetCapsuleComponent))
  (Variables|Default|SetaxisInput AxisValue)
  (if (Variables|Default|GetisFlying)
    (if (> AxisValue 0.0)
      (Class|PrimitiveComponent|SetPhysicsAngularVelocityinRadians (Variables|Collision|GetCapsuleComponent) "0, 0, 0" false "None")
      (Transformation|AddLocalRotation _capsulecomponent "-6.000000, 0, 0" false false)
      (elif (not (== AxisValue 0.0))
        (Class|PrimitiveComponent|SetPhysicsAngularVelocityinRadians (Variables|Collision|GetCapsuleComponent) "0, 0, 0" false "None")
        (Transformation|AddLocalRotation _capsulecomponent "6.000000, 0, 0" false false)))
    (else
      (bind _output_get (Variables|Default|Setdirection (.x (Math|Vector|Normalize (Math|Vector|GetUpVector _returnvalue) 1.0))))
      (Variables|Default|Setforce (* (Math|Vector|GetForwardVector _returnvalue) AxisValue))
      (if (>= (* AxisValue _output_get) 0.0)
        (Variables|Default|Setforce (* (Variables|Default|Getforce) 1.8e+02))
        (else
          (Variables|Default|Setforce (* (* (Variables|Default|Getforce) 1.8e+03) (Math|Float|Absolute(Float) (Variables|Default|Getdirection))))))
      (Physics|AddForce (Variables|Default|Gethead) (Variables|Default|Getforce) "None" true)
      (Variables|Default|SetlastSpin 0))))

(fn ConstructionScript)

(fn IsExcessivelyInclined
  (if (> (Math|Float|Absolute(Float) (.x (Math|Vector|Normalize (Math|Vector|GetUpVector (Transformation|GetActorRotation)) 1.0))) 0.9)
    (return true)
    (else
      (return false))))

(fn MakeRagdoll
  (bind _mesh (Variables|Character|GetMesh))
  (if (not (Variables|Default|GetisFlying))
    (if (not (Variables|Default|GetisDeath))
      (Collision|SetCollisionProfileName _mesh "Ragdoll" true :!class /Script/Engine.PrimitiveComponent)
      (Physics|SetSimulatePhysics _mesh true)
      (Audio|PlaySoundatLocation "/Game/Kenny/Sound/CE_DeathSound.CE_DeathSound" (Transformation|GetActorLocation) "0, 0, 0" 1.0 1.0 0.0 0 0 0)
      (Variables|Default|SetisDeath true))))

(fn RunDieObserver
  (bind _isexcessivelyinclined (CallFunction|IsExcessivelyInclined))
  (if _isexcessivelyinclined
    (CallFunction|MakeRagdoll)))